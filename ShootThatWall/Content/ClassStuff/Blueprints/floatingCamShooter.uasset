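; Floating camera shooter pawn that moves in its view plane and fires projectiles with the left mouse button.
; Horizontal and Vertical axes add movement along the control rotation's right and up vectors, with no forward movement.
; Each click spawns a Projectile just ahead along the control rotation, then a short Delay leads to destroying the most recently spawned one.
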(event Input|AxisEvents|InputAxisVertical
  (params (AxisValue :type Float%20%28single-precision%29))
  (Pawn|Input|AddMovementInput (Math|Vector|GetUpVector (Pawn|GetControlRotation :!class /Script/Engine.Pawn)) AxisValue false))

(event Input|AxisEvents|InputAxisHorizontal
  (params (AxisValue :type Float%20%28single-precision%29))
  (Pawn|Input|AddMovementInput (Math|Vector|GetRightVector (Pawn|GetControlRotation :!class /Script/Engine.Pawn)) AxisValue false))

(event Input|MouseEvents|LeftMouseButton
  (params (Key :type Key%20Structure :default "AnyKey"))
  (bind _returnvalue (Pawn|GetControlRotation :!class /Script/Engine.Pawn))
  (:Pressed
    (bind _returnvalue_2 (Game|SpawnActorfromClass "/Game/ClassStuff/Blueprints/projectile.projectile_C" (Math|Transform|MakeTransform (+ (* (Math|Vector|GetForwardVector _returnvalue) 1e+02) (Transformation|GetActorLocation)) _returnvalue) "Undefined" 0 0))
    (Utilities|FlowControl|Delay 0.5)
    (Actor|DestroyActor _returnvalue_2)))

(fn ConstructionScript)